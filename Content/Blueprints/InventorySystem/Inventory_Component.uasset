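; Actor component that holds an inventory, sized to SlotsQuantity at BeginPlay, and toggles its on-screen UI.
; ToggleInventory creates an Inventory_Widget bound to the component and anchors it on the BP_ThirdPersonCharacter HUD canvas, or removes it if open.
; Each toggle switches input mode between UI-only and game-only and shows or hides the cursor.
; Adding and stacking items are unimplemented stubs, with AddToInventory always returning false.
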(event `self.ReceiveBeginPlay`
  (`KismetArrayLibrary.Array_Resize` (`self.Inventory`) (`self.Slots Quantity`)))

(fn `Add To Inventory`
  (returns (Success :type Boolean))
  (return false))

(fn `Add to Stack`)

(fn `Create Stack`)

(fn `Toggle Inventory`
  (bind _returnvalue (`GameplayStatics.GetPlayerController` 0))
  (bind _inventory_ui (`self.Inventory UI`)
    (:`then`
      (`Widget.RemoveFromParent` _inventory_ui)
      (set `self.Inventory UI` null)
      (`WidgetBlueprintLibrary.SetInputMode_GameOnly` _returnvalue)
      (set `PlayerController.bShowMouseCursor` false _returnvalue))
    (:`else`
      (bind _returnvalue_2 (`|CreateWidget` "/Game/Blueprints/InventorySystem/UI/Inventory_Widget.Inventory_Widget_C" null self (`self.Inventory Name`)))
      (bind _output_get (set `self.Inventory UI` _returnvalue_2))
      (bind _asbp_third_person_character (cast `/Game/ThirdPerson/Blueprints/BP_ThirdPersonCharacter` (`GameplayStatics.GetPlayerCharacter` 0)))
      (bind _returnvalue_3 (`CanvasPanel.AddChildToCanvas` (`/Game/Blueprints/InventorySystem/InventoryHud.Canvas` (`/Game/ThirdPerson/Blueprints/BP_ThirdPersonCharacter.Inventory Hud` _asbp_third_person_character)) _output_get))
      (`CanvasPanelSlot.SetAutoSize` _returnvalue_3 true)
      (`CanvasPanelSlot.SetAlignment` _returnvalue_3 (0.5 0.5))
      (`CanvasPanelSlot.SetAnchors` _returnvalue_3 (make `Anchors` (0.4 0.1) (1.0 1.0)))
      (`WidgetBlueprintLibrary.SetInputMode_UIOnlyEx` _returnvalue _output_get)
      (set `PlayerController.bShowMouseCursor` true _returnvalue))))