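; Interactable door Blueprint that swings open and closed on alternate Interact events.
; A timeline drives the Door component's relative yaw between closed and -105 degrees, playing forward to open and in reverse to close.
; An IsDoorMoving flag ignores further interaction until the timeline finishes, and DoorOpening tracks the direction.
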(event `/Game/Blueprints/Interaction_IE.Interact`
  (if (not (`self.Is Door Moving?`))
    (set `self.Is Door Moving?` true)
    (bind _output_get (set `self.Door Opening` (not (`self.Door Opening`))))
    (if _output_get
      (bind (_direction _newtrack_1) (`Timeline|Door Timeline` :!label _label)
        (:`Update`
          (`SceneComponent.K2_SetRelativeRotation` (`self.Door`) (`KismetMathLibrary.MakeRotator` 0.0 0.0 (`KismetMathLibrary.Lerp` 0.0 -105.0 _newtrack_1)) false false)
          (set `self.Is Finished` true))
        (:`Finished`
          (set `self.Is Door Moving?` false)))
      (else
        (goto _label :!via `Reverse`)))))

(fn `UserConstructionScript`)