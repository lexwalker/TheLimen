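; Master_Item is a base pickup actor that the player collects by interacting with it.
; Interact checks ItemStructure: addable items go to the player's Inventory_Component, while others flagged as beneficial call PickUpBenefits.
; The actor destroys itself only when the chosen path reports success.
; PickUpBenefits returns false here, apparently a hook for child items to override, and Interact also prints the CanbeAdded flag.
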(event `/Game/Blueprints/Interaction_IE.Interact`
  (bind (_item_structure_itemname _item_structure_itemdesctiprion _item_structure_canbeadded_ _item_structure_itemicon _item_structure_isstackable_ _item_structure_ispickupbenefitial) (break `/Game/Blueprints/InventorySystem/Item_Structure` (`self.Item Structure`)))
  (bind _asbp_third_person_character (cast `/Game/ThirdPerson/Blueprints/BP_ThirdPersonCharacter` (`GameplayStatics.GetPlayerCharacter` 0)))
  (`KismetSystemLibrary.PrintText` (`KismetTextLibrary.Conv_BoolToText` _item_structure_canbeadded_))
  (if _item_structure_canbeadded_
    (bind _success (`/Game/Blueprints/InventorySystem/Inventory_Component.Add To Inventory` (`self.GetComponentByClass` _asbp_third_person_character "/Game/Blueprints/InventorySystem/Inventory_Component.Inventory_Component_C")))
    (if _success
      (`self.K2_DestroyActor` :!label _label))
    (elif _item_structure_ispickupbenefitial
      (bind _success_2 (`self.Pick Up Benefits`))
      (if _success_2
        (goto _label)))))

(fn `Pick Up Benefits`
  (returns (Success :type Boolean))
  (return false))

(fn `UserConstructionScript`)